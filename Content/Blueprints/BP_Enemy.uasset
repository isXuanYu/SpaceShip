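; BP_Enemy is an enemy ship actor that handles its randomized coloring, spawn-in scaling and explosion visuals.
; SetColor picks body and wing colors independently from a four-color palette, applies them through a dynamic material instance, and plays a timeline that drives actor scale.
; SpawnExplosion spawns a particle emitter at the ship's location, passing in the two stored colors so the explosion matches the ship.
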(event EventBeginPlay)

(event Collision|EventActorBeginOverlap
  (params (OtherActor :type Actor%20Object%20Reference)))

(event EventTick
  (params (DeltaSeconds :type Float%20%28single-precision%29)))

(event EventSetColor
  (Variables|Default|SetBodyColorIndex (Math|Random|RandomIntegerinRange 0 3))
  (Variables|Default|SetWingColorIndex (Math|Random|RandomIntegerinRange 0 3))
  (bind _returnvalue (Rendering|Material|CreateDynamicMaterialInstance "/Game/SpaceshipBattle/Materials/M_Base_Ship.M_Base_Ship" "None" "None" :!class /Script/Engine.KismetMaterialLibrary))
  (Rendering|Material|SetVectorParameterValue _returnvalue "Color1" (Utilities|Select :Index (Variables|Default|GetBodyColorIndex) :Option%200 "(R=1.000000,G=0.000000,B=0.000000,A=1.000000)" :Option%201 "(R=0.000000,G=1.000000,B=0.000000,A=1.000000)" :Option%202 "(R=0.000000,G=0.000000,B=1.000000,A=1.000000)" :Option%203 "(R=0.800000,G=0.678470,B=0.000000,A=1.000000)") :!class /Script/Engine.MaterialInstanceDynamic)
  (Variables|Default|SetPrimaryColor (Utilities|Select :Index (Variables|Default|GetBodyColorIndex) :Option%200 "(R=1.000000,G=0.000000,B=0.000000,A=1.000000)" :Option%201 "(R=0.000000,G=1.000000,B=0.000000,A=1.000000)" :Option%202 "(R=0.000000,G=0.000000,B=1.000000,A=1.000000)" :Option%203 "(R=0.800000,G=0.678470,B=0.000000,A=1.000000)"))
  (Rendering|Material|SetVectorParameterValue _returnvalue "Color2" (Utilities|Select :Index (Variables|Default|GetWingColorIndex) :Option%200 "(R=1.000000,G=0.000000,B=0.000000,A=1.000000)" :Option%201 "(R=0.000000,G=1.000000,B=0.000000,A=1.000000)" :Option%202 "(R=0.000000,G=0.000000,B=1.000000,A=1.000000)" :Option%203 "(R=0.800000,G=0.678470,B=0.000000,A=1.000000)") :!class /Script/Engine.MaterialInstanceDynamic)
  (Variables|Default|SetSecondryColor (Utilities|Select :Index (Variables|Default|GetWingColorIndex) :Option%200 "(R=1.000000,G=0.000000,B=0.000000,A=1.000000)" :Option%201 "(R=0.000000,G=1.000000,B=0.000000,A=1.000000)" :Option%202 "(R=0.000000,G=0.000000,B=1.000000,A=1.000000)" :Option%203 "(R=0.800000,G=0.678470,B=0.000000,A=1.000000)"))
  (Rendering|Material|SetMaterial (Variables|Default|GetShipSM) 0 _returnvalue)
  (bind _scale (Timeline|SpawScaleTimeline Play)
    (:Update
      (Transformation|SetActorScale3D (Math|Conversions|ToVector(Float) _scale)))))

(event EventSpawnExplosion
  (bind _returnvalue (Effects|SpawnEmitteratLocation "/Game/ParticleSystem/PS_Explosion.PS_Explosion" (Transformation|GetActorLocation)))
  (Effects|Components|ParticleSystem|SetColorParameter _returnvalue "PrimaryColor" (Variables|Default|GetPrimaryColor))
  (Effects|Components|ParticleSystem|SetColorParameter _returnvalue "SecondryColor" (Variables|Default|GetSecondryColor)))

(fn ConstructionScript)